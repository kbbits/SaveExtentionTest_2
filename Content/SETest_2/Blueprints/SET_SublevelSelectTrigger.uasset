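; Trigger volume that selects the active sublevel anchor, which SET_PlayerController uses for ball spawning.
; When player 0's pawn begins overlap, it assigns MySublevelAnchor to the controller and asynchronously streams in LoadOtherSubLevel if one is named.
; On end overlap it clears the anchor only if it is still its own; it does not unload the streamed level.
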(event `self.CollisionComponent.OnComponentBeginOverlap`
  (params (OverlappedComponent :type "PrimitiveComponent Object Reference") (OtherActor :type "Actor Object Reference") (OtherComp :type "PrimitiveComponent Object Reference") (OtherBodyIndex :type Integer) (bFromSweep :type Boolean) (SweepResult :type "HitResult Structure (by ref)"))
  (if (== OtherActor (`GameplayStatics.GetPlayerPawn` 0))
    ;[1 1 1] Set Sublevel Anchor. Used in PlayerController for ball spawning
    (bind _asset_player_controller (cast `/Game/SETest_2/Blueprints/SET_PlayerController` (`GameplayStatics.GetPlayerController` 0)))
    (set `/Game/SETest_2/Blueprints/SET_PlayerController.CurrentSublevelAnchor` (`self.MySublevelAnchor`) _asset_player_controller)
    ;[1 1 1] Load Subllevel, if any
    (if (!= (`self.LoadOtherSubLevel`) "None")
      (`GameplayStatics.LoadStreamLevel` (`self.LoadOtherSubLevel`) true))))

(event `self.CollisionComponent.OnComponentEndOverlap`
  (params (OverlappedComponent :type "PrimitiveComponent Object Reference") (OtherActor :type "Actor Object Reference") (OtherComp :type "PrimitiveComponent Object Reference") (OtherBodyIndex :type Integer))
  (if (== OtherActor (`GameplayStatics.GetPlayerPawn` 0))
    ;[1 1 1] Clear Sublevel Anchor on PlayerController.
    (bind _asset_player_controller (cast `/Game/SETest_2/Blueprints/SET_PlayerController` (`GameplayStatics.GetPlayerController` 0)))
    (if (== (`/Game/SETest_2/Blueprints/SET_PlayerController.CurrentSublevelAnchor` _asset_player_controller) (`self.MySublevelAnchor`))
      (set `/Game/SETest_2/Blueprints/SET_PlayerController.CurrentSublevelAnchor` null _asset_player_controller))))

(fn `UserConstructionScript`)