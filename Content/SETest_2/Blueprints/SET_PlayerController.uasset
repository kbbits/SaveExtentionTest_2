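; Player controller for a save system test scene that creates the main HUD and handles debug keys for ball spawning, saving, loading and quitting.
; Balls spawn ahead of and above the pawn, either owned by the current sublevel anchor with its color, or unowned in gold for the persistent level.
; Save and load act on the save manager's current slot and print success or failure.
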(event `self.ReceiveBeginPlay`
  (bind _returnvalue (`|CreateWidget` "/Game/SETest_2/UI/SET_MainHUD.SET_MainHUD_C" self))
  (bind _output_get (set `self.MainHUD` _returnvalue))
  (`UserWidget.AddToViewport` _output_get 0))

(event `Key|B`
  (params (Key :type "Key Structure"))
  (bind _currentsublevelanchor (`self.CurrentSublevelAnchor`))
  ;[1 1 1] Drop actors (balls) with data in them.
  (:`Pressed`
    (if (and (`self.SpawnInSublevel`) (`KismetSystemLibrary.IsValid` (`self.CurrentSublevelAnchor`)))
      ;;[1 1 1] Spawn into sublevel (anchor as owner) and set color from sublevel anchor
      (`|SpawnActorFromClass` "/Game/SETest_2/Blueprints/Actors/SET_Ball.SET_Ball_C" (`self.GetBallSpawnTransform`) "Undefined" "OverrideRootScale" _currentsublevelanchor (`/Game/SETest_2/Blueprints/Actors/SET_SublevelAnchor.SublevelColor` _currentsublevelanchor) null)
      (else
        ;;[1 1 1] Spawn into persistent level
        (`|SpawnActorFromClass` "/Game/SETest_2/Blueprints/Actors/SET_Ball.SET_Ball_C" (`self.GetBallSpawnTransform`) "Undefined" "OverrideRootScale" null (struct :`R` 1.0 :`G` 0.83763 :`A` 1.0) null)))))

(event `Key|K`
  (params (Key :type "Key Structure"))
  ;[1 1 1] Save / Load
  (:`Pressed`
    (`SaveManager.BPSaveCurrentSlot` :`self` (subsystem `SaveManager`)
      (:`Continue`
        (`KismetSystemLibrary.PrintString` "Save successful" true true (struct :`G` 1.0 :`B` 0.029325 :`A` 1.0)))
      (:`Failed`
        (`KismetSystemLibrary.PrintString` "Save failed" true true (struct :`R` 1.0 :`G` 0.009094 :`A` 1.0))))))

(event `Key|L`
  (params (Key :type "Key Structure"))
  ;[1 1 1] Save / Load
  (:`Pressed`
    (`SaveManager.BPReloadCurrentSlot` (subsystem `SaveManager`)
      (:`Continue`
        (`KismetSystemLibrary.PrintString` "Load successful" true true (struct :`G` 1.0 :`B` 0.029325 :`A` 1.0)))
      (:`Failed`
        (`KismetSystemLibrary.PrintString` "Load failed" true true (struct :`R` 1.0 :`G` 0.009094 :`A` 1.0))))))

(event `Key|X`
  (params (Key :type "Key Structure"))
  (:`Pressed`
    (if (`self.IsInputKeyDown` "LeftShift")
      (`KismetSystemLibrary.QuitGame` null "Quit"))))

(fn `GetBallSpawnTransform`
  (returns (Transform :type "Transform Structure"))
  ;[1 1 1] Drop the ball short distance in "Front" of pawn.
  (return (`KismetMathLibrary.MakeTransform` (+ (`self.K2_GetActorLocation` (`self.K2_GetPawn`)) (`KismetMathLibrary.MakeVector` (.x (* (`self.GetActorForwardVector` (`self.K2_GetPawn`)) 180.0)) (.y (* (`self.GetActorForwardVector` (`self.K2_GetPawn`)) 180.0)) 200.0)))))

(fn `UserConstructionScript`)