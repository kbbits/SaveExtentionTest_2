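; SET_Ball is a save/load test actor: a randomly scaled ball holding struct data that changes when the player hits it.
; On BeginPlay it fills empty MyData with randomly picked rows from the GameState's data table and applies MyColor to the sphere.
; Player hits increment and print each struct's TestInt, throttled by a one-second DoOnce.
; The SaveManager's OnGameLoaded event reapplies the color after loading.
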(event `self.ReceiveBeginPlay`
  (`|ExecutionSequence`
    (:`then_0`
      ;[1 1 1] Init GameState var
      (bind _asset_game_state (cast `/Game/SETest_2/Blueprints/SET_GameState` (`GameplayStatics.GetGameState`)))
      (bind _output_get (set `self.MyGameState` _asset_game_state)))
    (:`then_1`
      ;[1 1 1] Init MyData with some data pulled from GameState data table.  Rows chosen randomly.
      (if (== (`KismetArrayLibrary.Array_Length` (`self.MyData`)) 0)
        (bind _outrownames (`DataTableFunctionLibrary.GetDataTableRowNames` (`/Game/SETest_2/Blueprints/SET_GameState.MyGameData` (`self.MyGameState`))))
        (for _ (range (+ (`KismetMathLibrary.RandomIntegerInRange` 0 (- (`KismetArrayLibrary.Array_Length` _outrownames) 1)) 1))
          (bind _returnvalue (`|GetDataTableRow` (`/Game/SETest_2/Blueprints/SET_GameState.MyGameData` (`self.MyGameState`)) (`|GetArrayItem` _outrownames (`KismetMathLibrary.RandomIntegerInRange` 0 (- (`KismetArrayLibrary.Array_Length` _outrownames) 1))))
            (:`then`
              ;;[1 1 1] Add a copy of struct from DataTable row
              (`KismetArrayLibrary.Array_Add` (`self.MyData`) (`|Copy` _returnvalue)))))))
    (:`then_2`
      ;[1 1 1] Bind to OnLoaded
      (add `SaveManager.OnGameLoaded` (subsystem `SaveManager`) (delegate `OnGameLoaded`)))
    (:`then_3`
      ;[1 1 1] Set color, for debug visibility
      (`MeshComponent.SetVectorParameterValueOnMaterials` (`self.Sphere`) "Color" (`KismetMathLibrary.Conv_LinearColorToVector` (`self.MyColor`)) :!label _label))))

(event `OnGameLoaded`
  (params (SlotInfo :type "SlotInfo Object Reference"))
  ;[1 1 1] Bind to OnLoaded
  (goto _label))

(event `self.Sphere.OnComponentHit`
  (params (HitComponent :type "PrimitiveComponent Object Reference") (OtherActor :type "Actor Object Reference") (OtherComp :type "PrimitiveComponent Object Reference") (NormalImpulse :type "Vector Structure") (Hit :type "HitResult Structure (by ref)"))
  (if (== (`GameplayStatics.GetPlayerPawn` 0) OtherActor)
    (`/Engine/EditorBlueprintResources/StandardMacros.DoOnce` false :!label _label_2
      (:`Completed`
        ;[1 1 1] Change some data in MyData. These changes should be saved/loaded.
        (for (_array_element _array_index) (`self.MyData`)
          (bind _structout (setmembers `TestStruct` :`StructRef` (`|GetArrayItem` (`self.MyData`) _array_index) :`TestInt` (+ (`.TestInt` (break `TestStruct` _array_element)) 1)))
          (bind (_name _testfloat _testint) (break `TestStruct` _structout))
          ;;[1 1 1] Print for debug
          (`KismetSystemLibrary.PrintString` (`KismetStringLibrary.BuildString_Int` (`KismetStringLibrary.Conv_NameToString` _name) ": " _testint)))
        ;[1 1 1] Allow another OnHit interaction after delay.
        (`KismetSystemLibrary.Delay` 1.0)
        (goto _label_2 :!via `Reset`)))))

(fn `UserConstructionScript`
  (`SceneComponent.SetWorldScale3D` (`self.Sphere`) (* (1.0 1.0 1.0) (`KismetMathLibrary.RandomFloatInRange` 0.25 1.0))))